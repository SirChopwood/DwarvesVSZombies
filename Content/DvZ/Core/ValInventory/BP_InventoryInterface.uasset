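; BP_InventoryInterface appears to be a Blueprint interface for the ValInventory system, declaring calls for inventory slots and item tooltips.
; Slot functions read an item, assign an item and set the displayed quantity.
; Tooltip functions build title and description data from previous stats, show a tooltip with title, description and stats, and hide it.
; All bodies are empty stubs with default returns, leaving behavior to implementers.
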(fn GetTooltipData
  (params (PreviousStats :type Array%20of%20S%20Tooltip%20Stat%20Structures))
  (return "" "" 0))

(fn HideTooltip
  (return false))

(fn GetItemfromSlot
  (return 0))

(fn SetItemtoSlot
  (params (Item :type BP%20Dv%20Z%20Item%20Base%20Object%20Reference))
  (return false))

(fn ShowTooltip
  (params (Title :type Text) (Description :type Text) (Stats :type Array%20of%20S%20Tooltip%20Stat%20Structures))
  (return false))

(fn SetDisplayQuantity
  (params (Amount :type Integer))
  (return false))