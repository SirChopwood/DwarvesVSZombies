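; Inventory item object that holds name, description, stack quantity and tiered enchantments.
; GetEnchantment searches the Enchantments list and returns the tier with its primary, secondary and tertiary values, indexed by tier minus one.
; GetTooltipData appends colored enchantment and quantity lines to the incoming stats, then returns them with title and description.
; Slot, display-quantity and tooltip show/hide functions are empty stubs.
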(fn GetEnchantment
  (params (Query :type PDA%20Enchantments%20Object%20Reference))
  (for _array_element (Variables|Default|GetEnchantments)
    (if (== (.enchantment _array_element) Query)
      (return true Query (.tier _array_element) (Utilities|Array|Get(acopy) (Variables|/Game/DvZ/Core/ValInventory/PDA_Enchantments.PDA_Enchantments_C|GetPrimaryValue (.enchantment _array_element)) (- (.tier _array_element) 1)) (Utilities|Array|Get(acopy) (Variables|/Game/DvZ/Core/ValInventory/PDA_Enchantments.PDA_Enchantments_C|GetSecondaryValue (.enchantment _array_element)) (- (.tier _array_element) 1)) (Utilities|Array|Get(acopy) (Variables|/Game/DvZ/Core/ValInventory/PDA_Enchantments.PDA_Enchantments_C|GetTertiaryValue (.enchantment _array_element)) (- (.tier _array_element) 1)))))
  (return false 0 0 0.0 0.0 0.0))

(fn GetItemfromSlot
  (return 0))

(fn GetTooltipData
  (params (PreviousStats :type Array%20of%20S%20Tooltip%20Stat%20Structures))
  (bind _enchantments (Variables|Default|GetEnchantments))
  (Utilities|FlowControl|Sequence
    (:then_0
      ;[0.01096 0.01161 0.0137] Get Enchantment Stats
      (if (> (Utilities|Array|Length _enchantments) 0)
        (for _array_element _enchantments
          (bind _formattedname (Default|GetFormattedName (.enchantment _array_element) (.tier _array_element)))
          (Utilities|Array|Add PreviousStats (Utilities|Struct|MakeS_TooltipStat (Utilities|Text|FormatText "- {Enchantment}" _formattedname) "(R=1.000000,G=0.498039,B=0.000000,A=0.800000)")))))
    (:then_1
      ;[0.01096 0.01161 0.0137] Get Quantity Stat
      (if (> (Variables|Default|GetMaxStackSize) 0)
        (Utilities|Array|Add PreviousStats (Utilities|Struct|MakeS_TooltipStat (Utilities|Text|FormatText "Quantity: {Current} / {Max}" (Variables|Default|GetQuantity) (Variables|Default|GetMaxStackSize)) "(R=1.000000,G=1.000000,B=1.000000,A=0.800000)"))))
    (:then_2
      (return (Variables|Default|GetName) (Variables|Default|GetDescription) PreviousStats))))

(fn HideTooltip
  (return false))

(fn SetDisplayQuantity
  (params (Amount :type Integer))
  (return false))

(fn SetItemtoSlot
  (params (Item :type BP%20Dv%20Z%20Item%20Base%20Object%20Reference))
  (return false))

(fn ShowTooltip
  (params (Title :type Text) (Description :type Text) (Stats :type Array%20of%20S%20Tooltip%20Stat%20Structures))
  (return false))