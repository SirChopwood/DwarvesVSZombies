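; Armour item object for the inventory system that supplies tooltip data and computes effective armour values.
; The tooltip adds the equipment slot before the parent's data, then appends durability tinted from red to green by the remaining ratio.
; GetArmourValues returns base armour, armour boosted by the Reinforced enchantment's percentage when present, and that result scaled by current over maximum durability.
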(fn GetTooltipData
  (params (PreviousStats :type Array%20of%20S%20Tooltip%20Stat%20Structures))
  (bind _maxdurability (Variables|Default|GetMaxDurability))
  (bind _currentdurability (Variables|Default|GetCurrentDurability))
  (Utilities|Array|Add PreviousStats (Utilities|Struct|MakeS_TooltipStat (Utilities|Text|FormatText "Slot: {Slot}" (Utilities|String|EnumtoString (Variables|Default|GetSlot))) "(R=0.000000,G=1.000000,B=1.000000,A=0.800000)"))
  (bind (_title _description _stats) (|CallParentFunction PreviousStats))
  (Utilities|Array|Add _stats (Utilities|Struct|MakeS_TooltipStat (Utilities|Text|FormatText "Durability: {Current} / {Max}" _currentdurability _maxdurability) (Math|Color|Lerp(LinearColor) "(R=1.000000,G=0.000000,B=0.000000,A=0.800000)" "(R=0.000000,G=1.000000,B=0.000000,A=0.800000)" (/ (Math|Conversions|ToFloat(Integer) _currentdurability) (Math|Conversions|ToFloat(Integer) _maxdurability)))))
  (return _title _description _stats))

(fn GetArmourValues
  (bind _basearmour (Variables|Default|GetBaseArmour))
  (bind _basearmour_2 (Variables|Default|GetBaseArmour))
  (bind _returnvalue (Math|Conversions|ToFloat(Integer) _basearmour))
  (bind (_found _enchantment _tier _primaryvalue) (CallFunction|GetEnchantment "/Game/DvZ/Core/ValInventory/DA_Enchantment_Reinforced.DA_Enchantment_Reinforced"))
  (if _found
    (return _returnvalue (* _returnvalue (+ (/ _primaryvalue 1e+02) 1.0)) (* (* _returnvalue (+ (/ _primaryvalue 1e+02) 1.0)) (/ (Variables|Default|GetCurrentDurability) (Variables|Default|GetMaxDurability))))
    (else
      (return (Math|Conversions|ToFloat(Integer) _basearmour_2) (Math|Conversions|ToFloat(Integer) _basearmour_2) (* _basearmour_2 (/ (Variables|Default|GetCurrentDurability) (Variables|Default|GetMaxDurability)))))))