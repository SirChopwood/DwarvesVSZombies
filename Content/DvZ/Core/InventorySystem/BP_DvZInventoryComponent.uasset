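; Base slot-based inventory component for DvZ that stores items in a fixed-size array and caches its owning character.
; On authority, BeginPlay sizes the array and runs setup hooks.
; Add, remove and swap events, meant for the server, edit slots through validating helpers, with swaps working across two components.
; Successful edits and the contents OnRep both fire an empty OnInventoryUpdate hook for client and server reactions.
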(event Custom|InitServer
  ;[0.01096 0.01161 0.0137] Handle Serverside Setup
  ;;[0.01096 0.01161 0.0137] Sets Array Length
  (Utilities|Array|SetArrayElem (Variables|Default|GetInventoryContents) (- (Variables|Default|GetInventorySize) 1) 0 true))

(event Custom|AddItem
  (params (Index :type Integer) (Item :type BP%20Dv%20Z%20Item%20Base%20Object%20Reference))
  ;[0.01096 0.01161 0.0137] Call Inventory Updates on Server
  (bind _success (CallFunction|AddItemtoContents Index Item))
  (if _success
    (CallFunction|OnInventoryUpdate)
    (else
      (Development|PrintString "Failed to Add Item" true true "(R=1.000000,G=0.004098,B=0.000000,A=1.000000)"))))

(event Custom|InitOwningClient
  ;[0.01096 0.01161 0.0137] Handle Client Setup
)

(event Custom|RemoveItem
  (params (Index :type Integer) (Item :type BP%20Dv%20Z%20Item%20Base%20Object%20Reference))
  ;[0.01096 0.01161 0.0137] Call Inventory Updates on Server
  (bind _success (CallFunction|RemoveItemfromContents Index Item))
  (if _success
    (CallFunction|OnInventoryUpdate)
    (else
      (Development|PrintString "Failed to Remove Item" true true "(R=1.000000,G=0.004098,B=0.000000,A=1.000000)"))))

(event Custom|SwapItems
  (params (SourceComponent :type BP%20Dv%20Z%20Inventory%20Component%20Object%20Reference) (SourceIndex :type Integer) (TargetComponent :type BP%20Dv%20Z%20Inventory%20Component%20Object%20Reference) (TargetIndex :type Integer))
  ;[0.01096 0.01161 0.0137] Call Inventory Updates on Server
  (bind _success (CallFunction|SwapItemsBetweenInventories SourceComponent SourceIndex TargetComponent TargetIndex))
  (if _success
    (CallFunction|OnInventoryUpdate SourceComponent)
    (CallFunction|OnInventoryUpdate TargetComponent)
    (else
      (Development|PrintString "Failed to Swap Items" true true "(R=1.000000,G=0.004098,B=0.000000,A=1.000000)"))))

(event Custom|OnInventoryUpdate
  ;[0.01096 0.01161 0.0137] Event to handle post update stuff on Client AND Server
)

(event EventBeginPlay
  (Utilities|FlowControl|Sequence
    (:then_0
      (bind _asbp_dv_zcharacter_base (Utilities|Casting|CastToBP_DvZCharacterBase (Components|GetOwner)))
      (Variables|Default|SetCharacterRef _asbp_dv_zcharacter_base))
    (:then_1
      (Networking|SwitchHasAuthority
        (:Authority
          (CallFunction|InitServer)
          (CallFunction|InitOwningClient))))))

(fn OnRepInventoryContents
  (CallFunction|OnInventoryUpdate))

(fn AddItemtoContents
  (params (Index :type Integer) (Item :type BP%20Dv%20Z%20Item%20Base%20Object%20Reference))
  (if (Math|Boolean|ANDBoolean (>= Index 0) (< Index (Variables|Default|GetInventorySize)) (not (Utilities|IsValid (Utilities|Array|Get(acopy) (Variables|Default|GetInventoryContents) Index))))
    (Utilities|Array|SetArrayElem (Variables|Default|GetInventoryContents) Index Item)
    (Development|PrintString (Utilities|String|ToString(Integer) Index))
    (return true)
    (else
      (return false))))

(fn RemoveItemfromContents
  (params (Index :type Integer) (Item :type BP%20Dv%20Z%20Item%20Base%20Object%20Reference))
  (bind _inventorycontents (Variables|Default|GetInventoryContents))
  ;[0.01096 0.01161 0.0137] Remove by Item
  (Utilities|IsValid Item
    (:Is%20Valid
      (if (Utilities|Array|ContainsItem _inventorycontents Item)
        (Utilities|Array|SetArrayElem _inventorycontents (Utilities|Array|FindItem _inventorycontents 0) 0)
        (return true)
        (else
          (return false))))
    (:Is%20Not%20Valid
      ;[0.01096 0.01161 0.0137] Remove by Index
      (if (and (>= Index 0) (< Index (Variables|Default|GetInventorySize)))
        (Utilities|Array|SetArrayElem _inventorycontents Index 0)
        (return true)
        (else
          (return false))))))

(fn SwapItemsBetweenInventories
  (params (SourceComponent :type BP%20Dv%20Z%20Inventory%20Component%20Object%20Reference) (SourceIndex :type Integer) (TargetComponent :type BP%20Dv%20Z%20Inventory%20Component%20Object%20Reference) (TargetIndex :type Integer))
  (LocalVariables|SetSourceItem (Utilities|Array|Get(acopy) (Variables|BP_DvZInventoryComponent_C|GetInventoryContents SourceComponent) SourceIndex))
  (LocalVariables|SetTargetItem (Utilities|Array|Get(acopy) (Variables|BP_DvZInventoryComponent_C|GetInventoryContents TargetComponent) TargetIndex))
  (bind _success (CallFunction|RemoveItemfromContents SourceComponent SourceIndex))
  (bind _success_2 (CallFunction|RemoveItemfromContents TargetComponent TargetIndex))
  (if (and _success_2 _success)
    (bind _success_3 (CallFunction|AddItemtoContents SourceComponent SourceIndex (LocalVariables|GetTargetItem)))
    (bind _success_4 (CallFunction|AddItemtoContents TargetComponent TargetIndex (LocalVariables|GetSourceItem)))
    (return (and _success_4 _success_3))
    (else
      (return false))))

(fn DebugPrintContents
  (params (TargetComponent :type BP%20Dv%20Z%20Inventory%20Component%20Object%20Reference))
  (bind _returnvalue (Utilities|IsValid TargetComponent))
  (bind _inventorycontents (Variables|Default|GetInventoryContents))
  (bind _inventorycontents_2 (Variables|BP_DvZInventoryComponent_C|GetInventoryContents TargetComponent))
  (bind _returnvalue_2 (select _returnvalue _inventorycontents_2 _inventorycontents))
  (Development|PrintString "=========================" true true "(R=1.000000,G=0.564395,B=0.000000,A=1.000000)" 1e+01)
  (for (_array_element _array_index) _returnvalue_2
    (Utilities|IsValid _array_element
      (:Is%20Valid
        (Development|PrintString (Utilities|String|ToString(Text) (Utilities|Text|FormatText "[{Slot}] {ItemName}" _array_index (Variables|/Game/DvZ/Core/InventorySystem/BP_DvZItemBase.BP_DvZItemBase_C|GetName _array_element))) true true "(R=1.000000,G=0.151048,B=0.000000,A=1.000000)" 1e+01))
      (:Is%20Not%20Valid
        (Development|PrintString (Utilities|String|ToString(Text) (Utilities|Text|FormatText "[{Slot}] Empty" _array_index)) true true "(R=1.000000,G=0.151048,B=0.000000,A=1.000000)" 1e+01))))
  (Development|PrintString (Utilities|String|ToString(Text) (Utilities|Text|FormatText "========================= 
PRINTING INVENTORY: {Name} with {Slots}/{Max} slots." (Utilities|GetDisplayName self) (Utilities|Array|Length _returnvalue_2) (Variables|Default|GetInventorySize))) true true "(R=1.000000,G=0.564395,B=0.000000,A=1.000000)" 1e+01))