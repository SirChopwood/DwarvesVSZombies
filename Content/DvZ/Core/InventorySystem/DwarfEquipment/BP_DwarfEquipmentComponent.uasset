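; Equipment component for dwarf characters, extending a parent inventory component with slot-based equipment and a toggleable menu.
; The menu widget is created on local possession; the toggle input FlipFlops it on screen, embedding the dwarf's inventory widget inside.
; Inventory updates refresh each equipment slot widget from the contents array, indexed by slot enum.
; Adding a valid item places it at its own slot type's index, rejecting non-equipment; invalid items keep the given index.
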(event Input|EnhancedActionEvents|EnhancedInputActionIA_ToggleInventory
  (params (ActionValue :type Boolean) (ElapsedSeconds :type Float%20%28double-precision%29) (TriggeredSeconds :type Float%20%28double-precision%29) (InputAction :type Input%20Action%20Object%20Reference :default "/Game/DvZ/Core/InventorySystem/CharacterInventory/IA_ToggleInventory.IA_ToggleInventory"))
  (bind _parentcharacter (Variables|Default|GetParentCharacter))
  (bind _equipmentmenu (Variables|Default|GetEquipmentMenu))
  (bind _asbp_dwarf_base (Utilities|Casting|CastToBP_DwarfBase _parentcharacter))
  (bind _bp_dwarfinventorycomponent (Variables|/Game/DvZ/Dwarves/BP_DwarfBase.BP_DwarfBase_C|GetBP_DwarfInventoryComponent _asbp_dwarf_base))
  (bind _inventorywidget (Variables|/Game/DvZ/Core/InventorySystem/CharacterInventory/BP_CharacterInventoryComponent.BP_CharacterInventoryComponent_C|GetInventoryWidget _bp_dwarfinventorycomponent))
  (Utilities|FlowControl|FlipFlop
    (:A
      (UserInterface|Viewport|AddtoViewport _equipmentmenu 0)
      (Class|ContentWidget|SetContent (Variables|/Game/DvZ/Core/InventorySystem/DwarfEquipment/WBP_DwarfMenu.WBP_DwarfMenu_C|GetInventorySlot _equipmentmenu) _inventorywidget))
    (:B
      (Widget|RemovefromParent _inventorywidget)
      (Widget|RemovefromParent (Variables|Default|GetEquipmentMenu)))))

(event EventOnPossessedbyLocalPlayer
  (|CallParentFunction)
  (bind _returnvalue (UserInterface|CreateWidget "/Game/DvZ/Core/InventorySystem/DwarfEquipment/WBP_DwarfMenu.WBP_DwarfMenu_C"))
  (Variables|Default|SetEquipmentMenu _returnvalue)
  (Development|PrintString "Hello"))

(event EventOnInventoryUpdate
  (|CallParentFunction)
  (Utilities|IsValid (Variables|Default|GetEquipmentMenu)
    (:Is%20Valid
      (bind _enumvalue (|ForEachE_EquipmentSlots)
        (:LoopBody
          (bind _slotwidget (Default|GetEquipmentSlot (Variables|Default|GetEquipmentMenu) _enumvalue))
          (Default|SetItemtoSlot _slotwidget (Utilities|Array|Get(acopy) (Variables|Default|GetInventoryContents) (Math|Conversions|ToInteger(Byte) _enumvalue))))))))

(fn AddItemtoContents
  (params (Index :type Integer) (Item :type BP%20Dv%20Z%20Item%20Base%20Object%20Reference))
  (Utilities|IsValid Item
    (:Is%20Valid
      (bind _asbp_dv_zequipment_base (Utilities|Casting|CastToBP_DvZEquipmentBase Item)
        (:then
          (bind _success (|CallParentFunction (Math|Conversions|ToInteger(Byte) (Variables|/Game/DvZ/Core/InventorySystem/DwarfEquipment/BP_DvZEquipmentBase.BP_DvZEquipmentBase_C|GetSlot _asbp_dv_zequipment_base)) Item))
          (return _success))
        (:CastFailed
          (return false))))
    (:Is%20Not%20Valid
      (bind _success_2 (|CallParentFunction Index Item))
      (return _success_2))))