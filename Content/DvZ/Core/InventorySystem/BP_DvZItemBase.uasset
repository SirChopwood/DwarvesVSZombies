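; BP_DvZItemBase is the base item Blueprint for the DvZ inventory system, supplying the data shown in an item's tooltip.
; GetTooltipData returns the item's name, description and a current/max quantity line, flagging stats for display only when the item can stack.
; The slot get/set and tooltip show/hide functions are empty stubs returning nothing or false, and the event graph has no active logic.
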(event EventBeginPlay)

(event Collision|EventActorBeginOverlap
  (params (OtherActor :type Actor%20Object%20Reference)))

(event EventTick
  (params (DeltaSeconds :type Float%20%28single-precision%29)))

(fn ConstructionScript)

(fn GetItemfromSlot
  (return 0))

(fn GetTooltipData
  (bind _maxstacksize (Variables|Default|GetMaxStackSize))
  (return (Variables|Default|GetName) (Variables|Default|GetDescription) (> _maxstacksize 1) (Utilities|Array|MakeArray (Utilities|Text|FormatText "Quantity: {Current} / {Max}" (Variables|Default|GetQuantity) _maxstacksize))))

(fn HideTooltip
  (return false))

(fn SetItemtoSlot
  (params (Item :type BP%20Dv%20Z%20Item%20Base%20Object%20Reference))
  (return false))

(fn ShowTooltip
  (params (Title :type Text) (Description :type Text) (ShowStats :type Boolean) (Stats :type Array%20of%20Texts))
  (return false))