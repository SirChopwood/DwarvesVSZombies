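; Equipment component for dwarf characters, an inventory subclass that holds one piece of equipment per slot type and shows it in a menu.
; AddItem forces each item into the index matching its slot enum, and swapping is disabled.
; The owning client creates the dwarf menu, whose slots refresh on every inventory update.
; Holding debug key E displays that menu with the dwarf's inventory widget embedded.
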(event EventInitOwningClient
  (|CallParentFunction)
  (bind _returnvalue (UserInterface|CreateWidget "/Game/DvZ/Core/InventorySystem/WBP_DwarfMenu.WBP_DwarfMenu_C"))
  (Variables|Default|SetEquipmentMenu _returnvalue))

(event EventAddItem
  (params (Index :type Integer) (Item :type BP%20Dv%20Z%20Item%20Base%20Object%20Reference))
  ;[0.01096 0.01161 0.0137] Force Equipment into correct slot
  (bind _asbp_dv_zequipment_base (Utilities|Casting|CastToBP_DvZEquipmentBase Item))
  (|CallParentFunction (Math|Conversions|ToInteger(Byte) (Variables|/Game/DvZ/Core/InventorySystem/BP_DvZEquipmentBase.BP_DvZEquipmentBase_C|GetSlot _asbp_dv_zequipment_base)) Item))

(event EventOnInventoryUpdate
  (|CallParentFunction)
  (Utilities|IsValid (Variables|Default|GetEquipmentMenu)
    (:Is%20Valid
      (bind _enumvalue (|ForEachE_EquipmentSlots)
        (:LoopBody
          (bind _slotwidget (Default|GetEquipmentSlot (Variables|Default|GetEquipmentMenu) _enumvalue))
          (Default|UpdateSlottedEquipment _slotwidget (.AsBP%20Dv%20ZEquipment%20Base (Utilities|Casting|CastToBP_DvZEquipmentBase (Utilities|Array|Get(acopy) (Variables|Default|GetInventoryContents) (Math|Conversions|ToInteger(Byte) _enumvalue))))))))))

(event EventSwapItems
  (params (Index1 :type Integer) (Index2 :type Integer))
  (Development|PrintString "You cannot swap Equipment" true true "(R=1.000000,G=0.000000,B=0.619255,A=1.000000)"))

(event Input|KeyboardEvents|DebugKeyE
  (params (Key :type Key%20Structure :default "None") (ActionValue :type Input%20Action%20Value%20Structure))
  (bind _returnvalue (Components|GetOwner))
  (bind _equipmentmenu (Variables|Default|GetEquipmentMenu))
  (bind _asbp_dwarf_base (Utilities|Casting|CastToBP_DwarfBase _returnvalue))
  (bind _bp_dwarfinventorycomponent (Variables|/Game/DvZ/Dwarves/BP_DwarfBase.BP_DwarfBase_C|GetBP_DwarfInventoryComponent _asbp_dwarf_base))
  (bind _inventorywidget (Variables|/Game/DvZ/Core/InventorySystem/BP_DwarfInventoryComponent.BP_DwarfInventoryComponent_C|GetInventoryWidget _bp_dwarfinventorycomponent))
  (:Pressed
    (UserInterface|Viewport|AddtoViewport _equipmentmenu 0)
    (Class|ContentWidget|SetContent (Variables|/Game/DvZ/Core/InventorySystem/WBP_DwarfMenu.WBP_DwarfMenu_C|GetInventorySlot _equipmentmenu) _inventorywidget))
  (:Released
    (Class|BPInventoryInterface|HideTooltip(Message) (Class|PanelWidget|GetAllChildren (Variables|/Game/DvZ/Core/InventorySystem/WBP_Inventory.WBP_Inventory_C|GetInventorySlotGrid _inventorywidget)))
    (Widget|RemovefromParent _inventorywidget)
    (Widget|RemovefromParent (Variables|Default|GetEquipmentMenu))))