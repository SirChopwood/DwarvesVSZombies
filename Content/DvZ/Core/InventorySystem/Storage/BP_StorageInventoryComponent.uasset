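; Inventory component for storage that opens a storage menu when a character interacts with it.
; Interact stores the character, creates WBP_StorageMenu for player controller 0 with this component as its source, initializes it with that character and adds it to the viewport.
; OnInventoryUpdate refreshes the menu's slots while the widget reference is valid.
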(event EventInteract
  (params (Character :type BP%20Dv%20Z%20Character%20Base%20Object%20Reference))
  (bind _output_get (Variables|Default|SetTargetCharacter Character))
  (bind _returnvalue (UserInterface|CreateWidget "/Game/DvZ/Core/InventorySystem/Storage/WBP_StorageMenu.WBP_StorageMenu_C" (Game|GetPlayerController 0) self))
  (bind _output_get_2 (Variables|Default|SetStorageMenu _returnvalue))
  (Default|InitWidget _output_get_2 _output_get)
  (UserInterface|Viewport|AddtoViewport _output_get_2 0))

(event EventOnInventoryUpdate
  (bind _storagemenu (Variables|Default|GetStorageMenu))
  (Utilities|IsValid _storagemenu
    (:Is%20Valid
      (Default|UpdateSlots _storagemenu))))