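; BP_DwarvenShortbow is a test inventory item for a bow that draws while primary action is held and fires on release.
; A looping timer builds the draw amount up to a cap, and release spawns a BP_ProjectileBase aimed at player 0's cursor hit point.
; Draw fraction scales only the forward spawn offset; no speed or damage is passed.
; Secondary action toggles aiming on the character's camera component.
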(event EventBeginPlay
  (|CallParentFunction) ; This node is disabled and will not be called.\nDrag off pins to build functionality.
)

(event Collision|EventActorBeginOverlap
  (params (OtherActor :type Actor%20Object%20Reference))
  (|CallParentFunction OtherActor) ; This node is disabled and will not be called.\nDrag off pins to build functionality.
)

(event EventTick
  (params (DeltaSeconds :type Float%20%28single-precision%29))
  (|CallParentFunction DeltaSeconds) ; This node is disabled and will not be called.\nDrag off pins to build functionality.
)

(fn ConstructionScript
  (|CallParentFunction))

(fn DrawStringTick
  (bind _output_get (Variables|Default|SetStringDrawnAmount (+ (Variables|Default|GetStringDrawnAmount) 0.1)))
  (if (>= _output_get (Variables|Default|GetStringDrawCap))
    (Development|PrintString "Bow Drawn" true true "(R=0.000000,G=1.000000,B=0.713224,A=1.000000)")
    (Utilities|Time|ClearandInvalidateTimerbyHandle (Variables|Default|GetStringDrawTimer))))

(fn ItemPrimaryActionEnd
  (params (Character :type BP%20Dv%20Z%20Character%20Base%20Object%20Reference))
  (bind _returnvalue (Transformation|GetActorLocation Character))
  (bind _stringdrawtimer (Variables|Default|GetStringDrawTimer))
  (Game|SpawnActorfromClass "/Game/DvZ/Core/CombatSystem/BP_ProjectileBase.BP_ProjectileBase_C" (Math|Transform|MakeTransform (+ (* (Transformation|GetActorForwardVector Character) 1e+02 (/ (Variables|Default|GetStringDrawnAmount) (Variables|Default|GetStringDrawCap))) _returnvalue) (Math|Rotator|FindLookatRotation _returnvalue (.impactpoint (.HitResult (Game|Player|GetHitResultUnderCursorbyChannel (Game|GetPlayerController 0) "TraceTypeQuery1" true)))) "1.000000,1.000000,1.000000") "Undefined" "MultiplyWithRoot" 0 Character Character)
  (Variables|Default|SetStringDrawnAmount 0.0)
  (if (Utilities|Time|IsValidTimerHandle _stringdrawtimer)
    (Utilities|Time|ClearandInvalidateTimerbyHandle _stringdrawtimer))
  (return true))

(fn ItemPrimaryActionStart
  (params (Character :type BP%20Dv%20Z%20Character%20Base%20Object%20Reference))
  (Development|PrintString "Draw String" true true "(R=0.159303,G=1.000000,B=0.000000,A=1.000000)")
  (bind _returnvalue (Utilities|Time|SetTimerbyEvent (EventDispatchers|CreateEvent :!event DrawStringTick) 0.1 true))
  (Variables|Default|SetStringDrawTimer _returnvalue)
  (return true))

(fn ItemSecondaryActionEnd
  (params (Character :type BP%20Dv%20Z%20Character%20Base%20Object%20Reference))
  (Variables|/Game/DvZ/Core/Character/BP_DvZCharacterCameraComponent.BP_DvZCharacterCameraComponent_C|SetIsAiming (Variables|/Game/DvZ/Core/Character/BP_DvZCharacterBase.BP_DvZCharacterBase_C|GetBP_DvZCharacterCameraComponent Character) false)
  (return true))

(fn ItemSecondaryActionStart
  (params (Character :type BP%20Dv%20Z%20Character%20Base%20Object%20Reference))
  (Variables|/Game/DvZ/Core/Character/BP_DvZCharacterCameraComponent.BP_DvZCharacterCameraComponent_C|SetIsAiming (Variables|/Game/DvZ/Core/Character/BP_DvZCharacterBase.BP_DvZCharacterBase_C|GetBP_DvZCharacterCameraComponent Character) true)
  (return true))