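; Dwarven Runeblade, a melee inventory item whose primary action plays a borrowed woodchopping montage and sets up a delayed arc swing; the secondary action is unused.
; StartSwingTick caches evenly spaced rotations across the arc around the character's facing and starts a looping timer.
; SwingTick consumes one rotation per step, sphere-tracing for pawns with debug drawing.
; Each target with a BP_DvZHealthComponent takes damage and knockback once per swing.
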(event EventBeginPlay
  (|CallParentFunction) ; This node is disabled and will not be called.\nDrag off pins to build functionality.
)

(event Collision|EventActorBeginOverlap
  (params (OtherActor :type Actor%20Object%20Reference))
  (|CallParentFunction OtherActor) ; This node is disabled and will not be called.\nDrag off pins to build functionality.
)

(event EventTick
  (params (DeltaSeconds :type Float%20%28single-precision%29))
  (|CallParentFunction DeltaSeconds) ; This node is disabled and will not be called.\nDrag off pins to build functionality.
)

(fn ConstructionScript
  (|CallParentFunction))

(fn SwingTick
  (bind _character (Variables|Runtime|GetCharacter))
  (bind _returnvalue (Transformation|GetActorLocation _character))
  (if (> (Utilities|Array|Length (Variables|SwingRuntime|GetSwingCache)) 0)
    (bind _outhits (Collision|MultiSphereTraceForObjects _returnvalue (+ _returnvalue (* (Math|Rotator|GetRotationXVector (Utilities|Array|Get(acopy) (Variables|SwingRuntime|GetSwingCache))) (Variables|SwingConfig|GetSwingSegmentLength))) (Variables|SwingConfig|GetSwingSegmentThickness) (Utilities|Array|MakeArray "ObjectTypeQuery3") false 0 "ForDuration"))
    (for _array_element _outhits
      (if (and (not (Utilities|Array|ContainsItem (Variables|SwingRuntime|GetSwingHitTargets) (.hitactor _array_element))) (!= (.hitactor _array_element) (Variables|Runtime|GetCharacter)))
        (Utilities|IsValid (Actor|GetComponentbyClass (.hitactor _array_element) "/Game/DvZ/Core/CombatSystem/BP_DvZHealthComponent.BP_DvZHealthComponent_C")
          (:Is%20Valid
            (Class|BPCombatInterface|DealDamage(Message) (Actor|GetComponentbyClass (.hitactor _array_element) "/Game/DvZ/Core/CombatSystem/BP_DvZHealthComponent.BP_DvZHealthComponent_C") (Variables|Runtime|GetCharacter) (Variables|SwingConfig|GetSwingDamage) (Variables|SwingConfig|GetSwingDamageType) 1e+01)
            (Utilities|Array|Add (Variables|SwingRuntime|GetSwingHitTargets) (.hitactor _array_element))))))
    (Utilities|Array|RemoveIndex (Variables|SwingRuntime|GetSwingCache))
    (else
      (Utilities|Time|ClearandInvalidateTimerbyHandle (Variables|SwingRuntime|GetSwingTimerRef)))))

(fn StartSwingTick
  (bind _singarcoffset (Variables|SwingConfig|GetSingArcOffset))
  (bind _character (Variables|Runtime|GetCharacter))
  (bind _returnvalue (Transformation|GetActorRotation _character))
  (bind _returnvalue_2 (Math|Rotator|CombineRotators _returnvalue (Math|Rotator|MakeRotator 0.0 0.0 _singarcoffset)))
  (bind (_roll _pitch) (Math|Rotator|BreakRotator _returnvalue_2))
  (Utilities|Array|Clear (Variables|SwingRuntime|GetSwingHitTargets))
  (LocalVariables|SetStarting%20Yaw (+ (.Yaw (Math|Rotator|BreakRotator _returnvalue_2)) (/ (Variables|SwingConfig|GetSwingArcWidth) 2.0)))
  (for _index (range 0 (Variables|SwingConfig|GetSwingSegmentCount))
    (Utilities|Array|Add (Variables|SwingRuntime|GetSwingCache) (Math|Rotator|MakeRotator _roll _pitch (- (LocalVariables|GetStarting%20Yaw) (* _index (/ (Variables|SwingConfig|GetSwingArcWidth) (Variables|SwingConfig|GetSwingSegmentCount)))))))
  (bind _returnvalue_3 (Utilities|Time|SetTimerbyEvent (EventDispatchers|CreateEvent :!event SwingTick) (/ (Variables|SwingConfig|GetSwingDuration) (Variables|SwingConfig|GetSwingSegmentCount)) true))
  (Variables|SwingRuntime|SetSwingTimerRef _returnvalue_3))

(fn ItemPrimaryActionEnd
  (params (Character :type BP%20Dv%20Z%20Character%20Base%20Object%20Reference))
  (return false))

(fn ItemPrimaryActionStart
  (params (Character :type BP%20Dv%20Z%20Character%20Base%20Object%20Reference))
  (bind _output_get (Variables|Runtime|SetCharacter Character))
  (Animation|PlayAnimMontage _output_get "/Game/Characters/Animations/AM_Woodchopping.AM_Woodchopping" 1.0 "None")
  (Utilities|Time|SetTimerbyEvent (EventDispatchers|CreateEvent :!event StartSwingTick) (Variables|SwingConfig|GetSwingDelay))
  (return true))

(fn ItemSecondaryActionEnd
  (params (Character :type BP%20Dv%20Z%20Character%20Base%20Object%20Reference))
  (return false))

(fn ItemSecondaryActionStart
  (params (Character :type BP%20Dv%20Z%20Character%20Base%20Object%20Reference))
  (return false))