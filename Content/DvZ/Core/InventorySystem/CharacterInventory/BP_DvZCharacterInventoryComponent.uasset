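; Character inventory component for DvZ that adds player inventory UI and hotbar selection on top of a parent inventory component.
; On local possession it creates the inventory widget and adds its input mapping context, then pushes contents to the widget on each update.
; Number-key input sets a clamped hotbar index used to return the current item.
; It creates and removes tooltip widgets, while slot, quantity and tooltip-data functions are empty stubs.
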(event Custom|SelectHotbarSlot
  (params (Index :type Integer))
  (bind _output_get (Variables|Default|SetCurrentHotbarIndex (Math|Integer|Clamp(Integer) Index 0 (- (Variables|Default|GetHotbarSize) 1))))
  (Development|PrintString (Utilities|String|ToString(Integer) _output_get)))

(event Input|EnhancedActionEvents|EnhancedInputActionIA_HotbarNumbers
  (params (ActionValue :type Float%20%28double-precision%29) (ElapsedSeconds :type Float%20%28double-precision%29) (TriggeredSeconds :type Float%20%28double-precision%29) (InputAction :type Input%20Action%20Object%20Reference :default "/Game/DvZ/Core/InventorySystem/CharacterInventory/IA_HotbarNumbers.IA_HotbarNumbers"))
  (CallFunction|SelectHotbarSlot (- (Math|Float|Round ActionValue) 1)))

(event EventOnPossessedbyLocalPlayer
  (|CallParentFunction)
  (bind _returnvalue (UserInterface|CreateWidget "/Game/DvZ/Core/InventorySystem/CharacterInventory/WBP_CharacterInventory.WBP_CharacterInventory_C" 0 self))
  (Variables|Default|SetInventoryWidget _returnvalue)
  (Input|AddMappingContext (PlayerController|LocalPlayerSubsystems|GetEnhancedInputLocalPlayerSubsystem (Game|GetPlayerController 0)) "/Game/DvZ/Core/InventorySystem/CharacterInventory/IMC_DvZCharacterInventory.IMC_DvZCharacterInventory" 0 "(bIgnoreAllPressedKeysUntilRelease=True,bForceImmediately=False,bNotifyUserSettings=False)"))

(event EventOnInventoryUpdate
  (bind _inventorywidget (Variables|Default|GetInventoryWidget))
  (|CallParentFunction)
  (Utilities|IsValid _inventorywidget
    (:Is%20Valid
      (Default|UpdateInventory _inventorywidget "(X=6.000000,Y=2.000000)" (Variables|Default|GetInventoryContents)))))

(fn GetCurrentHotbarItem
  (return (Utilities|Array|Get(acopy) (Variables|Default|GetInventoryContents) (Math|Integer|Clamp(Integer) (Variables|Default|GetCurrentHotbarIndex) 0 (- (Variables|Default|GetHotbarSize) 1)))))

(fn GetItemfromSlot
  (return 0))

(fn GetTooltipData
  (params (PreviousStats :type Array%20of%20S%20Tooltip%20Stat%20Structures))
  (return "" "" 0))

(fn HideTooltip
  (Utilities|IsValid (Variables|Default|GetCurrentTooltip)
    (:Is%20Valid
      (Widget|RemovefromParent (Variables|Default|GetCurrentTooltip))
      (Variables|Default|SetCurrentTooltip 0)
      (return true))
    (:Is%20Not%20Valid
      (return false))))

(fn SetDisplayQuantity
  (params (Amount :type Integer))
  (return false))

(fn SetItemtoSlot
  (params (Item :type BP%20Dv%20Z%20Item%20Base%20Object%20Reference))
  (return false))

(fn ShowTooltip
  (params (Title :type Text) (Description :type Text) (Stats :type Array%20of%20S%20Tooltip%20Stat%20Structures))
  (bind _returnvalue (UserInterface|CreateWidget "/Game/DvZ/Core/InventorySystem/CharacterInventory/WBP_CharacterInventoryTooltip.WBP_CharacterInventoryTooltip_C"))
  (bind _output_get (Variables|Default|SetCurrentTooltip _returnvalue))
  (Default|UpdateTooltip _output_get Title Description Stats)
  (return true))