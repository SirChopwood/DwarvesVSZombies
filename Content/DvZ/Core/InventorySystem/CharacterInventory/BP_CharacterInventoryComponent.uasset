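; Character inventory component for DvZ that connects a character's inventory to its UI.
; On local player possession it creates the inventory widget with itself as owning component and adds the inventory input mapping context.
; Inventory updates push the contents to that widget as a fixed-size grid.
; It also creates and removes item tooltip widgets, while the slot item, tooltip data and display quantity functions are empty stubs.
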(event EventOnPossessedbyLocalPlayer
  (|CallParentFunction)
  (bind _returnvalue (UserInterface|CreateWidget "/Game/DvZ/Core/InventorySystem/CharacterInventory/WBP_CharacterInventory.WBP_CharacterInventory_C" 0 self))
  (Variables|Default|SetInventoryWidget _returnvalue)
  (Input|AddMappingContext (PlayerController|LocalPlayerSubsystems|GetEnhancedInputLocalPlayerSubsystem (Game|GetPlayerController 0)) "/Game/DvZ/Core/InventorySystem/CharacterInventory/IMC_DvZCharacterInventory.IMC_DvZCharacterInventory" 0 "(bIgnoreAllPressedKeysUntilRelease=True,bForceImmediately=False,bNotifyUserSettings=False)"))

(event EventOnInventoryUpdate
  (bind _inventorywidget (Variables|Default|GetInventoryWidget))
  (|CallParentFunction)
  (Utilities|IsValid _inventorywidget
    (:Is%20Valid
      (Default|UpdateInventory _inventorywidget "(X=6.000000,Y=2.000000)" (Variables|Default|GetInventoryContents)))))

(fn GetItemfromSlot
  (return 0))

(fn GetTooltipData
  (return "" "" 0))

(fn HideTooltip
  (Utilities|IsValid (Variables|Default|GetCurrentTooltip)
    (:Is%20Valid
      (Widget|RemovefromParent (Variables|Default|GetCurrentTooltip))
      (Variables|Default|SetCurrentTooltip 0)
      (return true))
    (:Is%20Not%20Valid
      (return false))))

(fn SetDisplayQuantity
  (params (Amount :type Integer))
  (return false))

(fn SetItemtoSlot
  (params (Item :type BP%20Dv%20Z%20Item%20Base%20Object%20Reference))
  (return false))

(fn ShowTooltip
  (params (Title :type Text) (Description :type Text) (Stats :type Array%20of%20S%20Tooltip%20Stat%20Structures))
  (bind _returnvalue (UserInterface|CreateWidget "/Game/DvZ/Core/InventorySystem/CharacterInventory/WBP_CharacterInventoryTooltip.WBP_CharacterInventoryTooltip_C"))
  (bind _output_get (Variables|Default|SetCurrentTooltip _returnvalue))
  (Default|UpdateTooltip _output_get Title Description Stats)
  (return true))