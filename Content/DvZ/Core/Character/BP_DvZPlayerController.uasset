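; Player controller for DvZ that handles dwarf class selection and pawn swapping.
; Possessing a pawn whose class is exactly BP_DwarfBase opens the WBP_DwarfSelection widget with the cursor shown and Game and UI input.
; ChangeClass forwards the chosen class to ChangeClassServer, which on authority destroys the current pawn, spawns the new one at a hardcoded location and possesses it.
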(event Custom|ChangeClass
  (params (Class :type Actor%20Class%20Reference))
  (CallFunction|ChangeClassServer Class))

(event Custom|ShowDwarfSelection
  (bind _returnvalue (UserInterface|CreateWidget "/Game/DvZ/Dwarves/WBP_DwarfSelection.WBP_DwarfSelection_C"))
  (UserInterface|Viewport|AddtoViewport _returnvalue 0)
  (Input|SetInputModeGameandUI self 0 "DoNotLock" false false)
  (Variables|Default|SetbShowMouseCursor true))

(event Custom|ChangeClassServer
  (params (Class :type Actor%20Class%20Reference))
  (Networking|SwitchHasAuthority
    (:Authority
      (Actor|DestroyActor (Pawn|GetControlledPawn))
      (bind _returnvalue (Game|SpawnActorfromClass Class (Math|Transform|MakeTransform "1000.000000,1000.000000,100.000000" "0.000000,0.000000,0.000000" "1.000000,1.000000,1.000000") "AdjustIfPossibleButAlwaysSpawn" "MultiplyWithRoot" self 0))
      (Pawn|Possess (.AsPawn (Utilities|Casting|CastToPawn _returnvalue))))))

(event EventPossess
  (params (PossessedPawn :type Pawn%20Object%20Reference))
  (if (== (Utilities|GetClass PossessedPawn) "/Game/DvZ/Dwarves/BP_DwarfBase.BP_DwarfBase_C")
    (CallFunction|ShowDwarfSelection)))

(fn ConstructionScript)