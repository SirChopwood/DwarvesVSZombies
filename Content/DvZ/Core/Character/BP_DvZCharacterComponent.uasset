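; BP_DvZCharacterComponent is a base component for DvZ characters that provides hooks for server and local-player setup.
; On BeginPlay it caches its owning BP_DvZCharacterBase, binds to controller changes and manually runs that handler if a controller is already present.
; The handler fires OnPossessedByLocalPlayer for locally controlled pawns, while authority instances then call BeginPlayServer.
; Both hook events are empty in this Blueprint.
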(event Custom|BeginPlayServer)

(event Custom|OnPossessedByLocalPlayer)

(event Custom|OnParentControllerChanged
  (params (Pawn :type Pawn%20Object%20Reference) (OldController :type Controller%20Object%20Reference) (NewController :type Controller%20Object%20Reference))
  (if (Pawn|IsLocallyControlled Pawn)
    (CallFunction|OnPossessedbyLocalPlayer)))

(event EventBeginPlay
  (Utilities|FlowControl|Sequence
    (:then_0
      (bind _asbp_dv_zcharacter_base (Utilities|Casting|CastToBP_DvZCharacterBase (Components|GetOwner)))
      (bind _output_get (Variables|Default|SetParentCharacter _asbp_dv_zcharacter_base))
      (Pawn|BindEventtoReceiveControllerChangedDelegate _output_get (EventDispatchers|CreateEvent :!event Custom|OnParentControllerChanged))
      (Utilities|IsValid (Pawn|GetController _output_get)
        (:Is%20Valid
          (CallFunction|OnParentControllerChanged _output_get 0 (Pawn|GetController _output_get)))))
    (:then_1
      (Networking|SwitchHasAuthority
        (:Authority
          (CallFunction|BeginPlayServer))))))