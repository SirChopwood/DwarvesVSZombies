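; Character component for DvZ that builds and drives a smoothed follow camera for the locally possessed character.
; On possession it creates a detached spring arm and camera, then enables Tick to interpolate position, input-driven zoom and stepped rotation.
; Tick follows CalculateTargetCameraPos, whose graph holds math, marked unused, for cursor-plane aim offset, zoom-scaled velocity prediction and idle sway.
; Right mouse toggles aiming while held; optional debug spheres show both positions.
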(event Input|EnhancedActionEvents|EnhancedInputActionIA_Zoom
  (params (ActionValue :type Float%20%28double-precision%29) (ElapsedSeconds :type Float%20%28double-precision%29) (TriggeredSeconds :type Float%20%28double-precision%29) (InputAction :type Input%20Action%20Object%20Reference :default "/Game/DvZ/Core/Character/IA_Zoom.IA_Zoom"))
  ;[0.01096 0.01161 0.0137] Controls for Camera Zoom
  (Variables|Config|SetTargetZoom (Math|Float|Clamp(Float) (+ (Variables|Config|GetTargetZoom) (* ActionValue -2e+01)) (Variables|Config|GetMinZoom) (Variables|Config|GetMaxZoom))))

(event Input|EnhancedActionEvents|EnhancedInputActionIA_Rotate
  (params (ActionValue :type Float%20%28double-precision%29) (ElapsedSeconds :type Float%20%28double-precision%29) (TriggeredSeconds :type Float%20%28double-precision%29) (InputAction :type Input%20Action%20Object%20Reference :default "/Game/DvZ/Core/Character/IA_Rotate.IA_Rotate"))
  ;[0.01096 0.01161 0.0137] Controls for Camera Zoom
  (Variables|Runtime|SetTargetCameraRotation (Math|Rotator|CombineRotators (Variables|Runtime|GetTargetCameraRotation) (* "0.000000,90.000000,0.000000" ActionValue))))

(event EventOnPossessedbyLocalPlayer
  ;[0.01096 0.01161 0.0137] Init Chain
  (bind _asbp_dv_zcharacter_base (Utilities|Casting|CastToBP_DvZCharacterBase (Components|GetOwner)))
  (Variables|Runtime|SetAs%20BP%20DvZ%20Character%20Base _asbp_dv_zcharacter_base)
  (Variables|Runtime|SetTargetCameraPosition (Transformation|GetActorLocation (Variables|Runtime|GetAs%20BP%20DvZ%20Character%20Base)))
  (bind _returnvalue (Game|AddComponentbyClass (Variables|Runtime|GetAs%20BP%20DvZ%20Character%20Base) "/Script/Engine.SpringArmComponent" false (Math|Transform|MakeTransform "0, 0, 0" (Variables|Runtime|GetTargetCameraRotation) "1.000000,1.000000,1.000000")))
  (bind _output_get (Variables|Default|SetSpringArm _returnvalue))
  (Transformation|DetachFromComponent _output_get "KeepRelative" "KeepRelative" "KeepRelative" true)
  (Variables|/Script/Engine.SpringArmComponent|SetTargetArmLength _output_get 1.2e+03)
  (Variables|/Script/Engine.SpringArmComponent|SetbDoCollisionTest _output_get false)
  (Variables|/Script/Engine.SpringArmComponent|SetbEnableCameraLag _output_get true)
  (Variables|/Script/Engine.SpringArmComponent|SetCameraLagSpeed _output_get 5.0)
  (Variables|/Script/Engine.SpringArmComponent|SetbInheritYaw _output_get false)
  (Variables|/Script/Engine.SpringArmComponent|SetbInheritRoll _output_get false)
  (bind _returnvalue_2 (Game|AddComponentbyClass (Variables|Runtime|GetAs%20BP%20DvZ%20Character%20Base) "/Script/Engine.CameraComponent" true))
  (bind _output_get_2 (Variables|Default|SetCamera _returnvalue_2))
  (Transformation|AttachComponentToComponent _output_get_2 _output_get "None" "SnapToTarget" "SnapToTarget" "SnapToTarget" true)
  (Components|Tick|SetComponentTickEnabled true))

(event EventTick
  (params (DeltaSeconds :type Float%20%28single-precision%29))
  (bind _returnvalue (Utilities|CalculateTargetCameraPos))
  (bind _springarm (Variables|Default|GetSpringArm))
  (if (and (Utilities|IsValid (Variables|Default|GetSpringArm)) (Utilities|IsValid (Variables|Default|GetCamera)))
    (Utilities|FlowControl|Sequence
      (:then_0
        ;[0.01096 0.01161 0.0137] Update Camera Location
        (bind _output_get (Variables|Runtime|SetTargetCameraPosition (Math|Interpolation|VInterptoConstant (Variables|Runtime|GetTargetCameraPosition) _returnvalue DeltaSeconds (* (Variables|/Script/Engine.CharacterMovementComponent|GetMaxWalkSpeed (Variables|/Script/Engine.Character|GetCharacterMovement (Variables|Runtime|GetAs%20BP%20DvZ%20Character%20Base))) (Variables|Config|GetVelocityPredictionBlendSpeed)))))
        (Transformation|SetWorldLocation (Variables|Default|GetSpringArm) _output_get false false)
        ;;[0.01096 0.01161 0.0137] Debug Draw Points
        (if (Variables|Config|GetShowDebug)
          (Rendering|Debug|DrawDebugSphere _returnvalue 1e+01 12 "(R=0.000000,G=0.342752,B=1.000000,A=1.000000)" 0.0 3.0)
          (Rendering|Debug|DrawDebugSphere _output_get 12.0 12 "(R=0.000000,G=1.000000,B=0.004749,A=1.000000)" 0.0 3.0)))
      (:then_1
        ;[0.01096 0.01161 0.0137] Update Camera Zoom
        (Variables|/Script/Engine.SpringArmComponent|SetTargetArmLength (Variables|Default|GetSpringArm) (Math|Interpolation|FInterpTo (Variables|/Script/Engine.SpringArmComponent|GetTargetArmLength (Variables|Default|GetSpringArm)) (Variables|Config|GetTargetZoom) DeltaSeconds (Variables|Config|GetZoomBlendSpeed))))
      (:then_2
        ;[0.01096 0.01161 0.0137] Update Camera Rotation
        (Transformation|SetWorldRotation _springarm (Math|Interpolation|RInterpTo (Transformation|GetWorldRotation _springarm) (Variables|Runtime|GetTargetCameraRotation) DeltaSeconds (Variables|Config|GetCameraRotationSpeed)) false false)))))

(event Input|MouseEvents|DebugKeyRightMouseButton
  (params (Key :type Key%20Structure :default "None") (ActionValue :type Input%20Action%20Value%20Structure))
  (:Pressed
    (Variables|Runtime|SetIsAiming true))
  (:Released
    (Variables|Runtime|SetIsAiming false)))