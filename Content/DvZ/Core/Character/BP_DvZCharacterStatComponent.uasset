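; BP_DvZCharacterStatComponent is a character component that holds a single numeric stat with current, minimum and maximum values.
; SetValue clamps the new value to that range and calls OnValueUpdated, while AddValue applies a delta through SetValue.
; RepNotify functions on all three values make the same update call, so replicated changes notify in the same way.
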(event Custom|SetValue
  (params (Value :type Float%20%28double-precision%29))
  (Variables|Default|SetCurrentValue (Math|Float|Clamp(Float) Value (Variables|Default|GetMinValue) (Variables|Default|GetMaxValue)))
  (Default|CallOnValueUpdated))

(event Custom|AddValue
  (params (Value :type Float%20%28double-precision%29))
  (CallFunction|SetValue (+ Value (Variables|Default|GetCurrentValue))))

(fn OnRepCurrentValue
  (Default|CallOnValueUpdated))

(fn OnRepMaxValue
  (Default|CallOnValueUpdated))

(fn OnRepMinValue
  (Default|CallOnValueUpdated))