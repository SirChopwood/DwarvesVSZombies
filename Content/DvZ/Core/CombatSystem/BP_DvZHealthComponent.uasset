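; BP_DvZHealthComponent is a character health component built on inherited value logic (CurrentValue, MaxValue, OnValueUpdated).
; On server begin play it binds value updates to set HealthState to one of three states: full, below max or zero.
; On possession by the local player it creates a red progress bar in the hotbar's health slot and refreshes it on value updates.
; Debug keys 3 and 4 add fixed amounts of health.
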(event Custom|UpdateBar
  (Default|UpdateBar (Variables|Default|GetStatBar) (Variables|Default|GetCurrentValue) (Variables|Default|GetMaxValue)))

(event Custom|OnValueUpdated_Event
  (bind _currentvalue (Variables|Default|GetCurrentValue))
  (Variables|Default|SetHealthState (select (== _currentvalue 0.0) "NewEnumerator3" (select (< _currentvalue (Variables|Default|GetMaxValue)) "NewEnumerator1" "NewEnumerator0"))))

(event EventBeginPlayServer
  (|CallParentFunction)
  (EventDispatchers|AssignOnValueUpdated (delegate Custom|OnValueUpdated_Event)))

(event EventOnPossessedbyLocalPlayer
  (bind _returnvalue (UserInterface|CreateWidget "/Game/DvZ/Core/WBP_Progressbar.WBP_Progressbar_C"))
  (bind _output_get (Variables|Default|SetStatBar _returnvalue))
  (Default|InitBar _output_get false (Utilities|Struct|MakeSlateColor "(R=1.000000,G=0.050980,B=0.050980,A=1.000000)" "UseColor_Specified"))
  (Widget|Panel|AddChild (Variables|/Game/DvZ/Core/Character/WBP_Hotbar.WBP_Hotbar_C|GetHealthBarSlot (Variables|/Game/DvZ/Core/Character/BP_DvZCharacterBase.BP_DvZCharacterBase_C|GetHotbarWidget (Variables|Default|GetParentCharacter))) _output_get)
  (EventDispatchers|AssignOnValueUpdated (delegate Custom|UpdateBar))
  (CallFunction|UpdateBar))

(event Input|KeyboardEvents|DebugKey3
  (params (Key :type Key%20Structure :default "None") (ActionValue :type Input%20Action%20Value%20Structure))
  (:Pressed
    (CallFunction|AddValue 15.0)))

(event Input|KeyboardEvents|DebugKey4
  (params (Key :type Key%20Structure :default "None") (ActionValue :type Input%20Action%20Value%20Structure))
  (:Pressed
    (CallFunction|AddValue 25.0)))