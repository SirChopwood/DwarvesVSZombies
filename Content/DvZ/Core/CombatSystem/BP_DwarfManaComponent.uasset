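; Mana stat component for DvZ dwarf characters, with regeneration driven by the character's armour.
; On the server, a looping timer adds mana from ManaRegenCurve, sampled by current armour mapped against its base value, and requires a BP_DwarfArmourComponent.
; On local possession, it creates a blue progress bar in the hotbar's mana slot and refreshes it whenever the value updates.
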(event Custom|OnManaRechargeTick
  (bind _armourcomponent (Variables|Default|GetArmourComponent))
  (CallFunction|AddValue (Math|Curves|GetFloatValue (Variables|Default|GetManaRegenCurve) (Math|Float|MapRangeClamped (Variables|/Game/DvZ/Core/Character/BP_DvZCharacterStatComponent.BP_DvZCharacterStatComponent_C|GetCurrentValue _armourcomponent) 0.0 (Variables|/Game/DvZ/Core/CombatSystem/BP_DwarfArmourComponent.BP_DwarfArmourComponent_C|GetBaseValue _armourcomponent) 0.0 8e+01))))

(event Custom|OnValueUpdated_Event
  (Default|UpdateBar (Variables|Default|GetStatBar) (Variables|Default|GetCurrentValue) (Variables|Default|GetMaxValue)))

(event EventBeginPlayServer
  (bind _parentcharacter (Variables|Default|GetParentCharacter)
    (:then
      (bind _output_get (Variables|Default|SetArmourComponent (Actor|GetComponentbyClass _parentcharacter "/Game/DvZ/Core/CombatSystem/BP_DwarfArmourComponent.BP_DwarfArmourComponent_C")))
      (Utilities|IsValid _output_get
        (:Is%20Valid
          (bind _returnvalue (Utilities|Time|SetTimerbyEvent (delegate Custom|OnManaRechargeTick) 0.2 true))
          (Variables|Default|SetManaTimer _returnvalue))
        (:Is%20Not%20Valid
          (Development|PrintString "Actor requires Health Component" true true "(R=1.000000,G=0.055224,B=0.000000,A=1.000000)"))))
    (:else
      (Development|PrintString "Component only works on DvZ Characters" true true "(R=1.000000,G=0.055224,B=0.000000,A=1.000000)"))))

(event EventOnPossessedbyLocalPlayer
  (bind _returnvalue (UserInterface|CreateWidget "/Game/DvZ/Core/WBP_Progressbar.WBP_Progressbar_C"))
  (bind _output_get (Variables|Default|SetStatBar _returnvalue))
  (Default|InitBar _output_get true (Utilities|Struct|MakeSlateColor "(R=0.011765,G=0.274510,B=0.745098,A=1.000000)" "UseColor_Specified"))
  (Widget|Panel|AddChild (Variables|/Game/DvZ/Core/Character/WBP_Hotbar.WBP_Hotbar_C|GetManaBarSlot (Variables|/Game/DvZ/Core/Character/BP_DvZCharacterBase.BP_DvZCharacterBase_C|GetHotbarWidget (Variables|Default|GetParentCharacter))) _output_get)
  (EventDispatchers|AssignOnValueUpdated (delegate Custom|OnValueUpdated_Event)))