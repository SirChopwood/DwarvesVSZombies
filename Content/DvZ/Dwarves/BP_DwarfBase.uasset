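; BP_DwarfBase is a dwarf base Blueprint with equipment and inventory components, whose graph holds only debug helpers for populating them.
; One debug key spawns a Dwarven Runeplate and adds it to the equipment component.
; The other spawns a randomly sized Ingot stack and a second Runeplate into fixed inventory slots.
; Both keys print a confirmation, and the construction script only calls its parent.
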(event Custom|DebugAddArmour
  (bind _returnvalue (Game|SpawnActorfromClass "/Game/DvZ/Core/InventorySystem/TestItems/BP_DwarvenRuneplate.BP_DwarvenRuneplate_C" (Math|Transform|MakeTransform "0, 0, 0" "0, 0, 0" "1.000000,1.000000,1.000000") "Undefined" "MultiplyWithRoot" 0 0))
  (Default|AddItem (Variables|Default|GetBP_DwarfEquipmentComponent) 0 _returnvalue))

(event Custom|DebugAddItems
  (bind _bp_dwarfinventorycomponent (Variables|Default|GetBP_DwarfInventoryComponent))
  (bind _returnvalue (Game|SpawnActorfromClass "/Game/DvZ/Core/InventorySystem/TestItems/BP_Ingot.BP_Ingot_C" (Math|Transform|MakeTransform "0, 0, 0" "0, 0, 0" "1.000000,1.000000,1.000000") "Undefined" "MultiplyWithRoot" 0 0))
  (Variables|/Game/DvZ/Core/InventorySystem/BP_DvZItemBase.BP_DvZItemBase_C|SetQuantity _returnvalue (Math|Random|RandomIntegerinRange 1 50))
  (Default|AddItem _bp_dwarfinventorycomponent 0 _returnvalue)
  (bind _returnvalue_2 (Game|SpawnActorfromClass "/Game/DvZ/Core/InventorySystem/TestItems/BP_DwarvenRuneplate.BP_DwarvenRuneplate_C" (Math|Transform|MakeTransform "0, 0, 0" "0, 0, 0" "1.000000,1.000000,1.000000") "Undefined" "MultiplyWithRoot" 0 0))
  (Default|AddItem _bp_dwarfinventorycomponent 4 _returnvalue_2))

(event Input|KeyboardEvents|DebugKey1
  (params (Key :type Key%20Structure :default "None") (ActionValue :type Input%20Action%20Value%20Structure))
  (:Pressed
    (CallFunction|DebugAddArmour)
    (Development|PrintString "Add Armour")))

(event Input|KeyboardEvents|DebugKey2
  (params (Key :type Key%20Structure :default "None") (ActionValue :type Input%20Action%20Value%20Structure))
  (:Pressed
    (CallFunction|DebugAddItems)
    (Development|PrintString "Add Items")))

(fn ConstructionScript
  (|CallParentFunction))